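; Game state Blueprint that tracks scores and player counts for the red, green, blue and purple teams.
; Paired setter events and getter functions switch on team color to write or read a separate variable for each team.
; BeginPlay caches the first player pawn as a BP_Player reference.
; The blue score's OnRep function is empty, and the debug prints of both sets of values are unconnected.
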(event `self.ReceiveTick`
  (params (DeltaSeconds :type "Float (single-precision)")))

(event `self.ReceiveBeginPlay`
  ;[1 0.2048 0] Get Player Ref
  (bind _asbp_player (cast `/Game/Blueprints/Player/BP_Player` (`GameplayStatics.GetPlayerPawn` 0)))
  (set `self.PlayerRef` _asbp_player))

(event `/Game/Blueprints/Game/BI_GameStateInterface.SetTeamScore`
  (params (TeamColor :type Byte) (Value :type Byte))
  ;[0.08461 0.1927 0.04225] Sets team score
  (switch `int` (`KismetMathLibrary.Conv_ByteToInt` TeamColor)
    (:`1`
      (set `self.TeamRedScore` Value))
    (:`2`
      (set `self.TeamGreenScore` Value))
    (:`3`
      (set `self.TeamBlueScore` Value))
    (:`4`
      (set `self.TeamPurpleScore` Value))))

(event `/Game/Blueprints/Game/BI_GameStateInterface.SetPlayerAmount`
  (params (`Team Color` :type String) (Value :type Byte))
  ;[0.02083 0 0.00251] Set Player Amount
  (switch `string` `Team Color`
    (:`RED`
      (set `self.PlayerInRedTeam` Value))
    (:`GREEN`
      (set `self.PlayersInGreenTeam` Value))
    (:`BLUE`
      (set `self.PlayersInBlueTeam` Value))
    (:`PURPLE`
      (set `self.PlayersInPurpleTeam` Value))))

(fn `GetPlayerAmount`
  (params (`Team Color` :type String))
  (returns (Return :type Byte))
  (switch `string` `Team Color`
    (:`RED`
      (return (`self.PlayerInRedTeam`)))
    (:`GREEN`
      (return (`self.PlayersInGreenTeam`)))
    (:`BLUE`
      (return (`self.PlayersInBlueTeam`)))
    (:`PURPLE`
      (return (`self.PlayersInPurpleTeam`)))))

(fn `GetTeamScore`
  (params (TeamColor :type Byte))
  (returns (Value :type Byte))
  (switch `int` (`KismetMathLibrary.Conv_ByteToInt` TeamColor)
    (:`1`
      (return (`self.TeamRedScore`)))
    (:`2`
      (return (`self.TeamGreenScore`)))
    (:`3`
      (return (`self.TeamBlueScore`)))
    (:`4`
      (return (`self.TeamPurpleScore`)))))

(fn `OnRep_TeamBlueScore`)

(fn `UserConstructionScript`)