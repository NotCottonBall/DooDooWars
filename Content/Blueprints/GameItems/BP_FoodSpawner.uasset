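; Food spawner actor that periodically spawns its configured food class at its Arrow's location.
; On BeginPlay it looks up that class's color in a map, tints the spotlight and a dynamic material's emissive, then starts a looping timer.
; Each tick of the timer calls RS_SpawnFood, which spawns only if a vertical Camera-channel line trace through the Arrow hits nothing.
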(event `self.ReceiveBeginPlay`
  (bind _value (`BlueprintMapLibrary.Map_Find` (`self.FoodTypeToColor`) (`self.Actor To Spawn`)))
  (`LightComponent.SetLightColor` (`self.SpotLight`) _value true)
  (bind _returnvalue (`PrimitiveComponent.CreateDynamicMaterialInstance` (`self.StaticMesh`) 0 null "None"))
  (bind _output_get (set `self.SpawnerMaterial` _returnvalue))
  (`MaterialInstanceDynamic.SetVectorParameterValue` _output_get "EmmisiveColor" _value)
  (`KismetSystemLibrary.K2_SetTimerDelegate` (delegate `CallEvent_SpawnFood`) (`self.TimeBeforeSpawn`) true))

(event `CallEvent_SpawnFood`
  (`self.RS_SpawnFood`))

(event `RS_SpawnFood`
  (`self.CheckIfFoodExistsOnSpawner`
    (:`false`
      (`|SpawnActorFromClass` (`self.Actor To Spawn`) (`KismetMathLibrary.MakeTransform` (`SceneComponent.K2_GetComponentLocation` (`self.Arrow`))) "Undefined" "MultiplyWithRoot" null null))))

(fn `SpawnFood`)

(fn `UserConstructionScript`)