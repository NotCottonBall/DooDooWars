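; Multiplayer player character for a team poop-kicking game, handling input, movement, health, HUD and menus.
; Eaten food adds calories, which sprinting and spawning DooDoo consume; DooDoo is kicked with quick or charged impulses.
; Server-to-multicast event pairs replicate kicks, montages, effects, head pitch, preset chat messages and surface-based footsteps that emit AI noise.
; Tick projects the focused DooDoo onto the screen for a HUD indicator.
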(event `EnhancedInput|/Game/Inputs/IA_ChatOptions1`
  (params (ActionValue :type Boolean) (ElapsedSeconds :type "Float (double-precision)") (TriggeredSeconds :type "Float (double-precision)") (InputAction :type "InputAction Object Reference" :default "/Game/Inputs/IA_ChatOptions1.IA_ChatOptions1"))
  ;[0.04161 0.1613 1] Send Chat SMS
  (:`Started`
    (`self.SendSMS` 0)))

(event `RS_SendChatSMS`
  (params (SMS_ID :type Byte))
  ;[0.04161 0.1613 1] Send Chat SMS
  (`self.MC_SendChatSMS` SMS_ID))

(event `EnhancedInput|/Game/Inputs/IA_ChatOptions2`
  (params (ActionValue :type Boolean) (ElapsedSeconds :type "Float (double-precision)") (TriggeredSeconds :type "Float (double-precision)") (InputAction :type "InputAction Object Reference" :default "/Game/Inputs/IA_ChatOptions2.IA_ChatOptions2"))
  ;[0.04161 0.1613 1] Send Chat SMS
  (:`Started`
    (`self.SendSMS` 1)))

(event `MC_SendChatSMS`
  (params (SMS_ID :type Byte))
  (bind _hud (`self.HUD`))
  ;[0.04161 0.1613 1] Send Chat SMS
  (switch `/Game/ENUMS/ENUM_ChatSMSID` (cast `/Game/ENUMS/ENUM_ChatSMSID` SMS_ID)
    (:`NewEnumerator0`
      (`/Game/UI/Widgets/HUD/WB_HUD.AddMsgToChatBox` _hud "" "Nice Shot"))
    (:`NewEnumerator1`
      (`/Game/UI/Widgets/HUD/WB_HUD.AddMsgToChatBox` _hud "" "Nice Pass"))
    (:`NewEnumerator2`
      (`/Game/UI/Widgets/HUD/WB_HUD.AddMsgToChatBox` _hud "" "Im Vomiting"))
    (:`NewEnumerator3`
      (`/Game/UI/Widgets/HUD/WB_HUD.AddMsgToChatBox` _hud "" "Im Disappointed"))))

(event `EnhancedInput|/Game/Inputs/IA_ChatOptions3`
  (params (ActionValue :type Boolean) (ElapsedSeconds :type "Float (double-precision)") (TriggeredSeconds :type "Float (double-precision)") (InputAction :type "InputAction Object Reference" :default "/Game/Inputs/IA_ChatOptions3.IA_ChatOptions3"))
  ;[0.04161 0.1613 1] Send Chat SMS
  (:`Started`
    (`self.SendSMS` 2)))

(event `EnhancedInput|/Game/Inputs/IA_ChatOptions4`
  (params (ActionValue :type Boolean) (ElapsedSeconds :type "Float (double-precision)") (TriggeredSeconds :type "Float (double-precision)") (InputAction :type "InputAction Object Reference" :default "/Game/Inputs/IA_ChatOptions4.IA_ChatOptions4"))
  ;[0.04161 0.1613 1] Send Chat SMS
  (:`Started`
    (`self.SendSMS` 3)))

(event `OC_HideIndicator`
  (bind (_returnvalue_roll _returnvalue_pitch _returnvalue_yaw) (`KismetMathLibrary.BreakRotator` (`self.GetControlRotation`)))
  (bind (_returnvalue_x _returnvalue_y) (`KismetMathLibrary.BreakVector2D` (`WidgetLayoutLibrary.GetViewportSize`)))
  (bind _focusdoodoo (`self.FocusDooDoo`))
  (bind _screenposition (`GameplayStatics.ProjectWorldToScreen` (`GameplayStatics.GetPlayerController` 0) (`self.K2_GetActorLocation` _focusdoodoo)))
  (bind (_returnvalue_roll_2 _returnvalue_pitch_2 _returnvalue_yaw_2) (`KismetMathLibrary.BreakRotator` (`KismetMathLibrary.FindLookAtRotation` (`self.K2_GetActorLocation`) (`self.K2_GetActorLocation` (`self.FocusDooDoo`)))))
  ;[0.3494 0.1629 1] Checking for doodoo position to display it on viewport
  (`/Engine/EditorBlueprintResources/StandardMacros.IsValid` _focusdoodoo
    (:`Is Valid`
      (set `/Game/UI/Widgets/HUD/WB_HUD.IndicatorPosition` (`KismetMathLibrary.MakeVector2D` (`KismetMathLibrary.FClamp` (`KismetMathLibrary.BreakVector2D` _screenposition) 0.0 _returnvalue_x) (`KismetMathLibrary.FClamp` (`.Y` (`KismetMathLibrary.BreakVector2D` _screenposition)) 0.0 _returnvalue_y)) (`self.HUD`))
      (set `/Game/UI/Widgets/HUD/WB_HUD.IndicatorAngle` (- _returnvalue_yaw_2 _returnvalue_yaw) (`self.HUD`)))
    (:`Is Not Valid`
      (message `/Game/UI/Widgets/HUD/BI_HUD.SetDisplayDooDooIndicator` (`self.HUD`) false))))

(event `self.ReceiveTick`
  (params (DeltaSeconds :type "Float (single-precision)"))
  ;[0.3494 0.1629 1] Checking for doodoo position to display it on viewport
  (`self.OC_HideIndicator`))

(event `EnhancedInput|/Game/Inputs/IA_Toggle`
  (params (ActionValue :type Boolean) (ElapsedSeconds :type "Float (double-precision)") (TriggeredSeconds :type "Float (double-precision)") (InputAction :type "InputAction Object Reference" :default "/Game/Inputs/IA_Toggle.IA_Toggle"))
  ;[0 0.3585 1] Other Triggers
  ;;[1 0.719 0.2142] DooDooIndicator
  (:`Started`
    (`self.OC_ToggleIndicator`)))

(event `OC_ToggleIndicator`
  ;[0 0.3585 1] Other Triggers
  ;;[1 0.719 0.2142] DooDooIndicator
  (`/Engine/EditorBlueprintResources/StandardMacros.FlipFlop`
    (:`A`
      (message `/Game/UI/Widgets/HUD/BI_HUD.SetDisplayDooDooIndicator` (`self.HUD`) true))
    (:`B`
      (message `/Game/UI/Widgets/HUD/BI_HUD.SetDisplayDooDooIndicator` (`self.HUD`) false))))

(event `EnhancedInput|/Game/Inputs/IA_Chat`
  (params (ActionValue :type Boolean) (ElapsedSeconds :type "Float (double-precision)") (TriggeredSeconds :type "Float (double-precision)") (InputAction :type "InputAction Object Reference" :default "/Game/Inputs/IA_Chat.IA_Chat"))
  (bind _returnvalue (`GameplayStatics.GetPlayerController` 0))
  ;[0 0.3585 1] Other Triggers
  ;;[1 0.05984 0.2097] Show chat menu
  (:`Started`
    (`/Engine/EditorBlueprintResources/StandardMacros.FlipFlop`
      (:`A`
        (bind _returnvalue_2 (`|CreateWidget` "/Game/UI/Widgets/InGameMenus/WB_Chat.WB_Chat_C" _returnvalue))
        (`UserWidget.AddToViewport` _returnvalue_2 0)
        (`WidgetBlueprintLibrary.SetInputMode_GameAndUIEx` _returnvalue _returnvalue_2 "DoNotLock" false)
        (set `PlayerController.bShowMouseCursor` true _returnvalue))
      (:`B`
        (`Widget.RemoveFromParent` _returnvalue_2)
        (`WidgetBlueprintLibrary.SetInputMode_GameOnly` _returnvalue)
        (set `PlayerController.bShowMouseCursor` false _returnvalue)))))

(event `EnhancedInput|/Game/Inputs/IA_GameInfo`
  (params (ActionValue :type Boolean) (ElapsedSeconds :type "Float (double-precision)") (TriggeredSeconds :type "Float (double-precision)") (InputAction :type "InputAction Object Reference" :default "/Game/Inputs/IA_GameInfo.IA_GameInfo"))
  ;[0 0.3585 1] Other Triggers
  ;;[1 0 0.42] game info menu
  (:`Started`
    (bind _returnvalue (`|CreateWidget` "/Game/UI/Widgets/InGameMenus/WB_GameInfo.WB_GameInfo_C" (`GameplayStatics.GetPlayerController` 0)))
    (`UserWidget.AddToViewport` _returnvalue 0))
  (:`Completed`
    (`Widget.RemoveFromParent` _returnvalue)))

(event `self.ReceiveBeginPlay`
  (bind _returnvalue (`GameplayStatics.GetPlayerController` 0))
  ;[1 0.6426 0.2226] Setup
  (bind _asplayer_controller (cast `PlayerController` _returnvalue))
  (bind _returnvalue_2 (pcsubsystem `EnhancedInputLocalPlayerSubsystem` _asplayer_controller))
  (`/Engine/EditorBlueprintResources/StandardMacros.IsValid` _returnvalue_2
    (:`Is Valid`
      (`EnhancedInputSubsystemInterface.AddMappingContext` _returnvalue_2 "/Game/Inputs/IMC_Main.IMC_Main" 0 (struct))
      (bind _asbc_player_hud (cast `/Game/UI/Widgets/HUD/BC_PlayerHUD` (`PlayerController.GetHUD` _returnvalue)))
      (set `self.HUD` (`/Game/UI/Widgets/HUD/BC_PlayerHUD.HUD_Ref` _asbc_player_hud)))))

(event `EnhancedInput|/Game/Inputs/IA_Pause`
  (params (ActionValue :type Boolean) (ElapsedSeconds :type "Float (double-precision)") (TriggeredSeconds :type "Float (double-precision)") (InputAction :type "InputAction Object Reference" :default "/Game/Inputs/IA_Pause.IA_Pause"))
  (bind _returnvalue (`GameplayStatics.GetPlayerController` 0))
  ;[0 0.3585 1] Other Triggers
  ;;[0.1302 0.05532 0.05144] Pause menu
  (:`Started`
    (bind _returnvalue_2 (`|CreateWidget` "/Game/UI/Widgets/InGameMenus/WB_PauseMenu.WB_PauseMenu_C" _returnvalue))
    (`UserWidget.AddToViewport` _returnvalue_2 0)
    (set `PlayerController.bShowMouseCursor` true _returnvalue)
    (`WidgetBlueprintLibrary.SetInputMode_UIOnlyEx` _returnvalue _returnvalue_2)))

(event `/Game/Blueprints/Player/BI_PlayerInterface.ShowWidget`
  (params (DisplayWidget :type Boolean))
  ;[1 0.9467 0] Player Interfaces
  ;;[1 1 1] Widget
  (set `/Game/UI/Widgets/HUD/WB_HUD.HintText` DisplayWidget (`self.HUD`)))

(event `/Game/Blueprints/Player/BI_PlayerInterface.SetFocusedDooDoo`
  (params (Actor :type "Actor Object Reference"))
  ;[1 0.9467 0] Player Interfaces
  ;;[1 0.3594 0.107] Focus DooDOo
  (set `self.FocusDooDoo` Actor))

(event `/Game/Blueprints/Player/BI_PlayerInterface.HurtPlayer`
  (params (HurtAmount :type "Float (double-precision)"))
  ;[1 0.9467 0] Player Interfaces
  ;;[0.9844 0.02527 0.1234] Set Health
  (bind _output_get (set `self.Health` (- (`self.Health`) HurtAmount)))
  (set `/Game/UI/Widgets/HUD/WB_HUD.CurrentHealth` _output_get (`self.HUD`)))

(event `EnhancedInput|/Game/Inputs/IA_Chat`
  (params (ActionValue :type Boolean) (ElapsedSeconds :type "Float (double-precision)") (TriggeredSeconds :type "Float (double-precision)") (InputAction :type "InputAction Object Reference" :default "/Game/Inputs/IA_Chat.IA_Chat"))
  (bind _returnvalue (`GameplayStatics.GetPlayerController` 0))
  ;[1 0.9467 0] Player Interfaces
  ;;[0.03875 0 0.2604] open chat menu (it just shows hints)
  (:`Started`
    (`/Engine/EditorBlueprintResources/StandardMacros.FlipFlop`
      (:`A`
        (set `self.Chatable` true)
        (bind _returnvalue_2 (`|CreateWidget` "/Game/UI/Widgets/InGameMenus/WB_Chat.WB_Chat_C" _returnvalue))
        (`UserWidget.AddToViewport` _returnvalue_2 0)
        (`WidgetBlueprintLibrary.SetInputMode_GameOnly` _returnvalue))
      (:`B`
        (set `self.Chatable` false)
        (`Widget.RemoveFromParent` _returnvalue_2)))))

(event `/Game/Blueprints/Player/BI_PlayerInterface.SetPlayerInfo`
  (params (InfoName :type String) (Value :type Byte))
  ;[1 0.9467 0] Player Interfaces
  ;;[0.1476 1 0.0534] Sets Player info
  (set `self.PlayerInfo` (`|MakeMap` InfoName Value)))

(event `/Game/Blueprints/Player/BI_PlayerInterface.PlayFootstepSounds`
  (bind _returnvalue (`self.K2_GetActorLocation`))
  ;[1 0.9467 0] Player Interfaces
  ;;[0.1898 0 1] Play Footstep Sound
  (bind (_outhit _returnvalue_2) (`KismetSystemLibrary.LineTraceSingle` _returnvalue (- _returnvalue (0.0 0.0 100.0)) "TraceTypeQuery1"))
  (if _returnvalue_2
    (`self.RS_PlayFootstepSound`)))

(event `EnhancedInput|/Game/Inputs/IA_PlayerMovement`
  (params (ActionValue :type "Vector2D Structure") (ElapsedSeconds :type "Float (double-precision)") (TriggeredSeconds :type "Float (double-precision)") (InputAction :type "InputAction Object Reference" :default "/Game/Inputs/IA_PlayerMovement.IA_PlayerMovement"))
  (bind (_returnvalue_roll _returnvalue_pitch _returnvalue_yaw) (`KismetMathLibrary.BreakRotator` (`self.GetControlRotation`)))
  (bind (_returnvalue_roll_2 _returnvalue_pitch_2 _returnvalue_yaw_2) (`KismetMathLibrary.BreakRotator` (`self.GetControlRotation`)))
  ;[0 0 0] Locomotion
  ;;[0 0.3313 1] Player Movement
  (:`Triggered`
    (if (`self.CanMove`)
      (if (`self.IsSprinting`)
        (if (> ActionValue_Y 0.0)
          (`self.AddMovementInput` (`KismetMathLibrary.GetForwardVector` (`KismetMathLibrary.MakeRotator` 0.0 0.0 _returnvalue_yaw)) ActionValue_Y :!label _label))
        (else
          (`self.AddMovementInput` (`KismetMathLibrary.GetRightVector` (`KismetMathLibrary.MakeRotator` _returnvalue_roll_2 0.0 _returnvalue_yaw_2)) ActionValue_X)
          (goto _label))))))

(event `/Game/Blueprints/Player/BI_PlayerInterface.SetPlayerTeamAmount_GameState`
  (params (TeamColor :type String) (IncrementDecrement :type Boolean))
  ;[1 0.9467 0] Player Interfaces
  ;;[1 1 1] change team amount in game state
  (`self.RS_SetPlayerAmount` TeamColor IncrementDecrement))

(event `EnhancedInput|/Game/Inputs/IA_Sprint`
  (params (ActionValue :type Boolean) (ElapsedSeconds :type "Float (double-precision)") (TriggeredSeconds :type "Float (double-precision)") (InputAction :type "InputAction Object Reference" :default "/Game/Inputs/IA_Sprint.IA_Sprint"))
  ;[0 0 0] Locomotion
  ;;[0.1147 0 1] Sprinting
  (:`Triggered`
    (`self.CheckAndDrainCalories`))
  (:`Started`
    (`self.RS_PlayFartingSound`))
  (:`Completed`
    (`self.StopSprinting`)))

(event `MC_SetWalkSpeed`
  (params (Speed :type "Float (double-precision)"))
  ;[0 0 0] Locomotion
  ;;[0.1147 0 1] Sprinting
  ;;;[0 0.934 1] Set Sprint Value For Everyone
  (set `CharacterMovementComponent.MaxWalkSpeed` Speed (`self.CharacterMovement`)))

(event `MC_PlayFootStepSound`
  ;[1 0.9467 0] Player Interfaces
  ;;[0.1898 0 1] Play Footstep Sound
  ;;;[1 0.4355 0] Play On Network
  (switch `EPhysicalSurface` (`GameplayStatics.GetSurfaceType` (stale `/Game/Blueprints/Player/BI_PlayerInterface.PlayFootstepSounds` _outhit))
    (:`SurfaceType1`
      (set `self.SoundOnFootstepHit` "/Game/SFX/HardFloor/SC_HardFloor.SC_HardFloor"))
    (:`SurfaceType2`
      (set `self.SoundOnFootstepHit` "/Game/SFX/MetalFloor/SC_MetalFloor.SC_MetalFloor"))
    (:`SurfaceType3`
      (set `self.SoundOnFootstepHit` "/Game/SFX/SoftFloor/SC_SoftFloor.SC_SoftFloor")))
  (bind (_bblockinghit _binitialoverlap _time _distance _location) (`GameplayStatics.BreakHitResult` (stale `/Game/Blueprints/Player/BI_PlayerInterface.PlayFootstepSounds` _outhit)))
  (`GameplayStatics.PlaySoundAtLocation` (`self.SoundOnFootstepHit`) _location (struct) 1.0 1.0 0.0 null null null null)
  (`AISense_Hearing.ReportNoiseEvent` _location 1.0 (`GameplayStatics.GetPlayerPawn` 0) 1000.0))

(event `EnhancedInput|/Game/Inputs/IA_CameraMovement`
  (params (ActionValue :type "Vector2D Structure") (ElapsedSeconds :type "Float (double-precision)") (TriggeredSeconds :type "Float (double-precision)") (InputAction :type "InputAction Object Reference" :default "/Game/Inputs/IA_CameraMovement.IA_CameraMovement"))
  (bind (_returnvalue_roll _returnvalue_pitch) (`KismetMathLibrary.BreakRotator` (`self.GetControlRotation`)))
  ;[0 0 0] Locomotion
  ;;[0.2384 1 0.4922] Head Movement
  (:`Triggered`
    ;;;[1 1 1] Moves Camera
    (`self.AddControllerYawInput` ActionValue_X)
    (`self.AddControllerPitchInput` ActionValue_Y)
    (`self.RS_SetPitch` _returnvalue_pitch)))

(event `RS_PlayFootstepSound`
  ;[1 0.9467 0] Player Interfaces
  ;;[0.1898 0 1] Play Footstep Sound
  ;;;[1 0.4355 0] Play On Network
  (`self.MC_PlayFootStepSound`))

(event `RS_SetPlayerAmount`
  (params (TeamColor :type String) (IncrementDecrement :type Boolean))
  ;[1 0.9467 0] Player Interfaces
  ;;[1 1 1] change team amount in game state
  (`/Engine/EditorBlueprintResources/ActorMacros.Switch Has Authority`
    (:`Authority`
      (if IncrementDecrement
        (`self.AddToTeamAmount` TeamColor)
        (else
          (`self.RemoveFromTeamAmount` TeamColor))))))

(event `CheckAndDrainCalories`
  ;[0 0 0] Locomotion
  ;;[0.1147 0 1] Sprinting
  ;;;[1 0.03805 0.1177] Calories--
  (if (and (> (`KismetMathLibrary.VSize` (`MovementComponent.Velocity` (`self.CharacterMovement`))) 0.0) (> (`self.Calories`) 0.0))
    (`self.ReduceCaloriesOnSprinting`)
    (`self.StartSprinting`)
    (else
      (`self.StopSprinting`))))

(event `RS_SetPitch`
  (params (RotationPitch :type "Float (double-precision)"))
  ;[0 0 0] Locomotion
  ;;[0.2384 1 0.4922] Head Movement
  ;;;[1 1 1] Set Pitch For Multiplayer
  (`self.MC_SetPitch` RotationPitch))

(event `MC_SetPitch`
  (params (RotationPitch :type "Float (double-precision)"))
  ;[0 0 0] Locomotion
  ;;[0.2384 1 0.4922] Head Movement
  ;;;[1 1 1] Set Pitch For Multiplayer
  (set `self.PlayerPitch` RotationPitch))

(event `RS_PlayFartingSound`
  ;[0 0 0] Locomotion
  (`self.MC_PlayFartingSound`))

(event `StartSprinting`
  ;[0 0 0] Locomotion
  ;;[0.1147 0 1] Sprinting
  ;;;[0.02701 1 0] Sprint Calls
  (`self.CheckAuthAndCallSprint` true (`self.RunSpeed`))
  (`self.MC_ToggleNiagaraSystem`))

(event `MC_ToggleNiagaraSystem`
  ;[0 0 0] Locomotion
  ;;[0.1147 0 1] Sprinting
  ;;;[1 0.1144 0] Niagara System
  (`self.ToggleNiagaraSystem` (`self.NS_Fart`)))

(event `StopSprinting`
  ;[0 0 0] Locomotion
  ;;[0.1147 0 1] Sprinting
  ;;;[0.02701 1 0] Sprint Calls
  (`self.CheckAuthAndCallSprint` false (`self.NormalSpeed`))
  (`self.MC_ToggleNiagaraSystem`))

(event `MC_PlayFartingSound`
  ;[0 0 0] Locomotion
  (`GameplayStatics.PlaySoundAtLocation` "/Game/SFX/Ensentials/farting.farting" (`SceneComponent.K2_GetComponentLocation` (`self.DooDooArrow`)) (struct) 1.0 1.0 0.0 null null null null))

(event `EnhancedInput|/Game/Inputs/IA_Kick`
  (params (ActionValue :type Boolean) (ElapsedSeconds :type "Float (double-precision)") (TriggeredSeconds :type "Float (double-precision)") (InputAction :type "InputAction Object Reference" :default "/Game/Inputs/IA_Kick.IA_Kick"))
  ;[1 0.6659 0.1437] Kick The DOODOO
  ;;[0 1 0.3557] Little Kick
  (:`Started`
    (if (not (`self.IsKickAiming`))
      (`self.RS_SetIsKickAiming` true)
      (set `self.CanMove` false)))
  (:`Completed`
    (set `self.KickStrength` 1000.0)
    (`self.KICK`)
    (set `self.CanMove` true)))

(event `EnhancedInput|/Game/Inputs/IA_KickAim`
  (params (ActionValue :type Boolean) (ElapsedSeconds :type "Float (double-precision)") (TriggeredSeconds :type "Float (double-precision)") (InputAction :type "InputAction Object Reference" :default "/Game/Inputs/IA_KickAim.IA_KickAim"))
  ;[1 0.6659 0.1437] Kick The DOODOO
  ;;[0 1 0.3557] Little Kick
  (:`Triggered`
    (`self.StartKickAim`))
  (:`Completed`
    (`self.KICK`)))

(event `RS_SetIsKickAiming`
  (params (Value :type Boolean))
  ;[1 0.6659 0.1437] Kick The DOODOO
  (set `self.IsKickAiming` Value))

(event `KICK`
  (bind _mesh (`self.Mesh`))
  (bind _returnvalue (`SceneComponent.K2_GetComponentLocation` _mesh))
  (bind (_returnvalue_roll _returnvalue_pitch _returnvalue_yaw) (`KismetMathLibrary.BreakRotator` (`SceneComponent.K2_GetComponentRotation` _mesh)))
  ;[1 0.6659 0.1437] Kick The DOODOO
  ;;[1 0.1874 0.9169] KICK
  (bind _outhits (`KismetSystemLibrary.SphereTraceMulti` :`Start` _returnvalue :`End` (+ _returnvalue (* (`KismetMathLibrary.GetForwardVector` (`KismetMathLibrary.MakeRotator` _returnvalue_roll _returnvalue_pitch (+ _returnvalue_yaw 90.0))) 100.0)) :`Radius` 35.0 :`TraceChannel` "TraceTypeQuery1" :`DrawDebugType` "Persistent"))
  (for _array_element _outhits
    (bind (_bblockinghit _binitialoverlap _time _distance _location _impactpoint _normal _impactnormal _physmat _hitactor) (`GameplayStatics.BreakHitResult` _array_element))
    (if (== _hitactor "/Game/Blueprints/Props/BP_DooDoo.BP_DooDoo")
      (break)))
  (`self.RS_AddImpulse` _hitactor (* (`SceneComponent.K2_GetComponentRotation` (`self.Camera`)) (`self.KickStrength`)))
  (`self.StopKickAim`))

(event `EnhancedInput|/Game/Inputs/IA_Interact`
  (params (ActionValue :type Boolean) (ElapsedSeconds :type "Float (double-precision)") (TriggeredSeconds :type "Float (double-precision)") (InputAction :type "InputAction Object Reference" :default "/Game/Inputs/IA_Interact.IA_Interact"))
  (bind _camera (`self.Camera`))
  (bind _returnvalue (`SceneComponent.K2_GetComponentLocation` _camera))
  ;[1 1 1] Bowel And Digestion
  ;;[0.001643 0.6875 0.3594] Eating Food
  (:`Started`
    (bind _outhit (`KismetSystemLibrary.LineTraceSingle` :`Start` _returnvalue :`End` (+ _returnvalue (* (`KismetMathLibrary.GetForwardVector` (`SceneComponent.K2_GetComponentRotation` _camera)) 200.0)) :`TraceChannel` "TraceTypeQuery1" :`DrawDebugType` "ForOneFrame"))
    (bind (_bblockinghit _binitialoverlap _time _distance _location _impactpoint _normal _impactnormal _physmat _hitactor) (`GameplayStatics.BreakHitResult` _outhit))
    (bind _rfoodvalue (message `/Game/Blueprints/Props/Food/BPI_Food.GetFoodValue` _hitactor))
    (`self.ConsumeFoodAndShowUI` _rfoodvalue)
    (`self.RS_DestroyObject` _hitactor)))

(event `EnhancedInput|/Game/Inputs/IA_Poop`
  (params (ActionValue :type Boolean) (ElapsedSeconds :type "Float (double-precision)") (TriggeredSeconds :type "Float (double-precision)") (InputAction :type "InputAction Object Reference" :default "/Game/Inputs/IA_Poop.IA_Poop"))
  ;[1 1 1] Bowel And Digestion
  ;;[0.6954 1 0.3112] Bowel Movement
  ;;;[0.07338 0.01239 1] Main Logic
  (:`Started`
    (`self.PerformCheck`)
    (set `self.CanMove` false)
    (`self.RS_DoDooDoo_Montage`)
    (`self.RS_DoDooDoo`)))

(event `MC_DestroyObject`
  (params (Actor :type "Actor Object Reference"))
  ;[1 1 1] Bowel And Digestion
  ;;[0.001643 0.6875 0.3594] Eating Food
  ;;;[1 0.1885 0] Destroying The Food Item
  (message `/Game/Blueprints/Props/Food/BPI_Food.DestroyFood` Actor))

(event `RS_DoDooDoo_Montage`
  ;[1 1 1] Bowel And Digestion
  ;;[0.6954 1 0.3112] Bowel Movement
  ;;;[0 0.1529 1] Play Montage
  (`self.MC_DoDooDoo_Montage`))

(event `MC_DoDooDoo_Montage`
  ;[1 1 1] Bowel And Digestion
  ;;[0.6954 1 0.3112] Bowel Movement
  ;;;[0 0.1529 1] Play Montage
  (`|PlayMontage` (`self.Mesh`) "/Game/Models/Player/Animations/Montages/AM_HumanoidJumpPoop.AM_HumanoidJumpPoop"
    (:`OnCompleted`
      (set `self.CanMove` true))))

(event `RS_DestroyObject`
  (params (Actor :type "Actor Object Reference"))
  ;[1 1 1] Bowel And Digestion
  ;;[0.001643 0.6875 0.3594] Eating Food
  ;;;[1 0.1885 0] Destroying The Food Item
  (`self.MC_DestroyObject` Actor))

(event `RS_AddImpulse`
  (params (PoopActor :type "Actor Object Reference") (KickAxis :type "Vector Structure"))
  ;[1 0.6659 0.1437] Kick The DOODOO
  ;;[1 0.1874 0.9169] KICK
  (`self.MC_AddImpulse` PoopActor KickAxis))

(event `MC_AddImpulse`
  (params (PoopActor :type "Actor Object Reference") (KickAxis :type "Vector Structure"))
  ;[1 0.6659 0.1437] Kick The DOODOO
  ;;[1 0.1874 0.9169] KICK
  (message `/Game/Blueprints/Props/BPI_DooDoo.GetKicked` PoopActor KickAxis))

(event `RS_DoDooDoo`
  ;[1 1 1] Bowel And Digestion
  ;;[0.6954 1 0.3112] Bowel Movement
  ;;;[1 0.3875 0.1658] Spawn The Poop
  (if (`self.HasAuthority`)
    (bind _returnvalue (`|SpawnActorFromClass` "/Game/Blueprints/Props/BP_DooDoo.BP_DooDoo_C" (`KismetMathLibrary.MakeTransform` (`SceneComponent.K2_GetComponentLocation` (`self.DooDooArrow`))) "Undefined" "MultiplyWithRoot" null null))
    (`self.MC_PoofDooDoo`)
    (`/Game/Blueprints/Player/BI_PlayerInterface.SetFocusedDooDoo` _returnvalue)))

(event `MC_PoofDooDoo`
  ;[1 1 1] Bowel And Digestion
  ;;[0.6954 1 0.3112] Bowel Movement
  ;;;[1 0.3875 0.1658] Spawn The Poop
  (`self.DooDooSpawnEffects`))

(fn `GetPlayerInfo`
  (returns (Return :type "Map of String to Byte"))
  (return (`self.PlayerInfo`)))

(fn `OnRep_IsKickAiming`)

(fn `SetTeamInfoInGameState`
  (switch `int` (`KismetMathLibrary.Conv_ByteToInt` (`BlueprintMapLibrary.Map_Find` (`self.PlayerInfo`) "Team"))
    (:`1`
      (`self.AddToTeamAmount` "RED"))
    (:`2`
      (`self.AddToTeamAmount` "GREEN"))
    (:`3`
      (`self.AddToTeamAmount` "BLUE"))
    (:`4`
      (`self.AddToTeamAmount` "PURPLE"))))

(fn `StartKickAim`
  (set `self.IsBusy` true)
  (set `self.CanMove` false)
  (set `self.KickStrength` (`KismetMathLibrary.FClamp` (+ (`self.KickStrength`) (* (`self.KickStrengthMultiplier`) (`GameplayStatics.GetWorldDeltaSeconds`))) 0.0 (`self.MaxKickStrength`)))
  (`self.RS_SetIsKickAiming` true))

(fn `StopKickAim`
  (set `self.IsBusy` false)
  (set `self.CanMove` true)
  (set `self.KickStrength` 0.0)
  (`self.RS_SetIsKickAiming` false))

(fn `UserConstructionScript`)