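; BP_DooDoo is a kickable dropping prop that poofs when it hits something in flight.
; Overlapping its sphere makes it the other actor's focused DooDoo, and a kick applies an impulse, then flags it airborne if a short downward trace misses.
; While airborne and moving, Tick sphere-traces for a hit, which routes destruction through RS to MC events for particles, sound and actor removal.
; It also records its spawn owner and reports zero food value.
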(event `/Game/Blueprints/Props/BPI_DooDoo.OnSpawn`
  (params (Actor :type "Actor Object Reference"))
  (set `self.SpawnOwner` Actor))

(event `self.ReceiveTick`
  (params (DeltaSeconds :type "Float (single-precision)"))
  (bind _returnvalue (`self.K2_GetActorLocation`))
  ;[0 1 0.5733] Check if the DooDoo Is Hitting Something after the player hits it
  (if (and (`self.IsInAir`) (>= (`KismetMathLibrary.VSize` (`self.GetVelocity`)) 0.1))
    (bind (_outhit _returnvalue_2) (`KismetSystemLibrary.SphereTraceSingle` :`Start` _returnvalue :`End` (- _returnvalue (10.0 0.0 0.0)) :`Radius` 30.0 :`TraceChannel` "TraceTypeQuery2" :`DrawDebugType` "Persistent"))
    (if _returnvalue_2
      (`self.RS_DestroyDooDoo`))))

(event `/Game/Blueprints/Props/BPI_DooDoo.GetKicked`
  (params (KickAxis :type "Vector Structure"))
  (bind _returnvalue (`self.K2_GetActorLocation`))
  ;[1 0 0.06858] Get Kicked
  (`PrimitiveComponent.AddImpulse` (`self.StaticMeshComponent`) KickAxis "None" true)
  (`KismetSystemLibrary.Delay` 0.1)
  (bind (_outhit _returnvalue_2) (`KismetSystemLibrary.LineTraceSingle` _returnvalue (- _returnvalue (0.0 0.0 10.0)) "TraceTypeQuery1"))
  (if (not _returnvalue_2)
    (set `self.IsInAir` true)))

(event `RS_DestroyDooDoo`
  ;[0.3265 1 0.4314] Destruction
  (`self.MC_DestroyDooDoo`))

(event `self.SphereCollision.OnComponentBeginOverlap`
  (params (OverlappedComponent :type "PrimitiveComponent Object Reference") (OtherActor :type "Actor Object Reference") (OtherComp :type "PrimitiveComponent Object Reference") (OtherBodyIndex :type Integer) (bFromSweep :type Boolean) (SweepResult :type "HitResult Structure (by ref)"))
  ;[1 0.1825 0.1228] Set this to the focusing doodoo
  (message `/Game/Blueprints/Player/BI_PlayerInterface.SetFocusedDooDoo` OtherActor self))

(event `MC_DestroyDooDoo`
  (bind _returnvalue (`self.K2_GetActorLocation`))
  ;[0.3265 1 0.4314] Destruction
  (`/Game/BF_GlobalFunctions.Poof` self _returnvalue (struct :`R` 0.114583 :`G` 0.05586 :`B` 0.018354 :`A` 1.0) true "/Game/VFX/NS_PoofEffect.NS_PoofEffect" (0.2 0.3) (0.1 0.2))
  (`GameplayStatics.PlaySoundAtLocation` "/Game/SFX/Ensentials/poof.poof" _returnvalue (struct) 1.0 1.0 0.0 null null null null))

(fn `GetFoodValue`
  (returns (RFoodValue :type "Float (double-precision)"))
  (return 0.0))

(fn `UserConstructionScript`)