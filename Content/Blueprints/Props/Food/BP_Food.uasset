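; BP_Food is a food prop that carries a food value, exposed through GetFoodValue.
; It loops an Actor Sequence from BeginPlay, and its Box overlap toggles a widget message on the actor entering or leaving.
; DestroyFood calls Poof to spawn a tinted Niagara puff at its location and destroy the actor.
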(event `self.ReceiveBeginPlay`
  (`MovieSceneSequencePlayer.PlayLooping` (`ActorSequenceComponent.SequencePlayer` (`self.ActorSequence`)) -1))

(event `/Game/Blueprints/Props/Food/BPI_Food.DestroyFood`
  (`/Game/BF_GlobalFunctions.Poof` self (`self.K2_GetActorLocation`) (`self.SmokeColor`) true "/Game/VFX/NS_PoofEffect.NS_PoofEffect" (0.1 0.3) (0.1 0.2)))

(event `self.Box.OnComponentBeginOverlap`
  (params (OverlappedComponent :type "PrimitiveComponent Object Reference") (OtherActor :type "Actor Object Reference") (OtherComp :type "PrimitiveComponent Object Reference") (OtherBodyIndex :type Integer) (bFromSweep :type Boolean) (SweepResult :type "HitResult Structure (by ref)"))
  (message `/Game/Blueprints/Player/BI_PlayerInterface.ShowWidget` OtherActor true))

(event `self.Box.OnComponentEndOverlap`
  (params (OverlappedComponent :type "PrimitiveComponent Object Reference") (OtherActor :type "Actor Object Reference") (OtherComp :type "PrimitiveComponent Object Reference") (OtherBodyIndex :type Integer))
  (message `/Game/Blueprints/Player/BI_PlayerInterface.ShowWidget` OtherActor false))

(fn `GetFoodValue`
  (returns (RFoodValue :type "Float (double-precision)"))
  (return (`self.FoodValue`)))

(fn `UserConstructionScript`)